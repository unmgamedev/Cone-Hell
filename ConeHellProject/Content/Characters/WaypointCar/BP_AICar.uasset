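; BP_AICar is an AI car that drives along a list of waypoints and halts while cones block it.
; After a start delay it plays engine and movement sounds, then Tick moves and rotates it straight toward the current waypoint without sweep.
; A detection box tracks overlapping BP_Cone actors to pause movement.
; Past the last waypoint, it plays a crash sound, notifies BP_TopDownGameMode and destroys itself rather than looping.
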(event `self.ReceiveBeginPlay`
  ;[0.05127 0.15 0.05127 0.502] Step 1
  ;; Car Delay
  (`KismetSystemLibrary.Delay` (`self.StartDelay`))
  (bind _output_get (set `self.CanMove` true))
  ;[0.15 0.08022 0.04231 0.502] Sound
  (`AudioComponent.Play` (`self.Engine Sound`) 0.0)
  (`AudioComponent.Play` (`self.Movement Sound`) 0.0))

(event `self.ReceiveTick`
  (params (DeltaSeconds :type "Float (single-precision)"))
  (bind _returnvalue (`self.K2_GetActorLocation`))
  (bind _returnvalue_2 (`self.K2_GetActorLocation` (`|GetArrayItem` (`self.Waypoints`) (`self.CurrentWaypointIndex`))))
  ;[0.05127 0.15 0.05127 0.502] Step 2
  ;; Checks if condition is true
  (if (and (stale `self.ReceiveBeginPlay` _output_get) (> (`KismetArrayLibrary.Array_Length` (`self.Waypoints`)) 0) (not (stale `self.ConeDetectionBox.OnComponentEndOverlap` _output_get)))
    ;; Apply movement & location
    (`self.K2_SetActorLocation` (+ (`self.K2_GetActorLocation`) (* (* (`KismetMathLibrary.GetDirectionUnitVector` _returnvalue _returnvalue_2) (`self.MoveSpeed`)) DeltaSeconds)))
    (`self.K2_SetActorRotation` (`KismetMathLibrary.FindLookAtRotation` _returnvalue _returnvalue_2))
    (if (<= (`KismetMathLibrary.Vector_Distance` _returnvalue _returnvalue_2) (`self.AcceptanceRadius`))
      ;[0.05127 0.15 0.05127 0.502] Step 3
      ;; Advance to Next Waypoint
      (bind _output_get (set `self.CurrentWaypointIndex` (+ (`self.CurrentWaypointIndex`) 1)))
      ;; Sends cars back to intial waypoint
      (if (>= (`self.CurrentWaypointIndex`) (`KismetArrayLibrary.Array_Length` (`self.Waypoints`)))
        (set `self.CurrentWaypointIndex` 0)
        ;[0.15 0.08022 0.04231 0.502] Sound
        (`GameplayStatics.SpawnSoundAtLocation` "/Game/TopDown/UI/Sounds/Car_Crash.Car_Crash" (`self.K2_GetActorLocation`) (struct) 1.0 1.0 0.0 null null)
        ;[0.15 0.08022 0.04231 0.502] Calculates cars being destroyed
        (bind _asbp_top_down_game_mode (cast `/Game/TopDown/Blueprints/BP_TopDownGameMode` (`GameplayStatics.GetGameMode`)))
        (`/Game/TopDown/Blueprints/BP_TopDownGameMode.CarDestroyed` _asbp_top_down_game_mode)
        ; Car Despawn
        (`self.K2_DestroyActor`)))))

(event `self.ConeDetectionBox.OnComponentBeginOverlap`
  (params (OverlappedComponent :type "PrimitiveComponent Object Reference") (OtherActor :type "Actor Object Reference") (OtherComp :type "PrimitiveComponent Object Reference") (OtherBodyIndex :type Integer) (bFromSweep :type Boolean) (SweepResult :type "HitResult Structure (by ref)"))
  ;[0.05127 0.15 0.05127 0.502] Step 1
  ;; Stop for Cones
  (bind _asbp_cone (cast `/Game/TopDown/Blueprints/BP_Cone` OtherActor))
  (`KismetArrayLibrary.Array_AddUnique` (`self.DetectedCones`) _asbp_cone)
  (set `self.StopForCone` true))

(event `self.ConeDetectionBox.OnComponentEndOverlap`
  (params (OverlappedComponent :type "PrimitiveComponent Object Reference") (OtherActor :type "Actor Object Reference") (OtherComp :type "PrimitiveComponent Object Reference") (OtherBodyIndex :type Integer))
  ;[0.05127 0.15 0.05127 0.502] Step 1
  ;; Stop for Cones
  (bind _asbp_cone (cast `/Game/TopDown/Blueprints/BP_Cone` OtherActor))
  (`KismetArrayLibrary.Array_RemoveItem` (`self.DetectedCones`) _asbp_cone)
  (bind _output_get (set `self.StopForCone` (> (`KismetArrayLibrary.Array_Length` (`self.DetectedCones`)) 0))))

(fn `UserConstructionScript`)