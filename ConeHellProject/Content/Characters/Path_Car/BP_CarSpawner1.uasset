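; Spawner actor that populates a referenced spline path with BP_AI_Car actors, up to a maximum count.
; BeginPlay starts a looping timer on SpawnCars, which re-arms it on each pass and spawns while the level-wide car count is below MaxCars.
; Each car is placed and oriented at SpawnIndex times Spacing along the spline and receives the spline reference.
; An unconnected spawn at the spline's first point is left unused.
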(event `SpawnCars`
  (bind _splineref (`self.SplineRef`))
  ; Spawner (based off spacing and time delay)
  (bind _outactors (`GameplayStatics.GetAllActorsOfClass` "/Game/Characters/Path_Car/BP_AI_Car.BP_AI_Car_C"))
  (`KismetSystemLibrary.K2_SetTimerDelegate` (delegate `SpawnCars`) (`self.SpawnDelay`) true :!label _label)
  (if (< (`KismetArrayLibrary.Array_Length` _outactors) (`self.MaxCars`))
    (`|SpawnActorFromClass` "/Game/Characters/Path_Car/BP_AI_Car.BP_AI_Car_C" (`KismetMathLibrary.MakeTransform` (`SplineComponent.GetLocationAtDistanceAlongSpline` (`/Game/Characters/Path_Car/BP_Path.Spline` _splineref) (* (`self.SpawnIndex`) (`self.Spacing`)) "World") (`SplineComponent.GetRotationAtDistanceAlongSpline` (`/Game/Characters/Path_Car/BP_Path.Spline` _splineref) (* (`self.SpawnIndex`) (`self.Spacing`)) "World")) "AlwaysSpawn" "MultiplyWithRoot" null (`self.SplineRef`) null)
    (set `self.SpawnIndex` (+ (`self.SpawnIndex`) 1))))

(event `self.ReceiveBeginPlay`
  ; Spawner (based off spacing and time delay)
  (goto _label))

(fn `UserConstructionScript`)