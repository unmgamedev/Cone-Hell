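; BP_AICar is an AI car actor that drives itself toward waypoint actors.
; Each Tick it moves in a straight line toward the current waypoint at MoveSpeed scaled by DeltaSeconds, and snaps its rotation to face it.
; Movement sets the transform directly without sweep, so collision does not block it.
; Within AcceptanceRadius, the waypoint index is set to a constant 1 rather than incremented, so it never advances further.
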(event `self.ReceiveTick`
  (params (DeltaSeconds :type "Float (single-precision)"))
  (bind _returnvalue (`self.K2_GetActorLocation`))
  (bind _returnvalue_2 (`self.K2_GetActorLocation` (`|GetArrayItem` (`self.Waypoints`) (`self.CurrentWaypointIndex`))))
  (if (> (`KismetArrayLibrary.Array_Length` (`self.Waypoints`)) 0)
    (`self.K2_SetActorLocation` (+ (`self.K2_GetActorLocation`) (* (* (`KismetMathLibrary.GetDirectionUnitVector` _returnvalue _returnvalue_2) (`self.MoveSpeed`)) DeltaSeconds)))
    (`self.K2_SetActorRotation` (`KismetMathLibrary.FindLookAtRotation` _returnvalue _returnvalue_2))
    (if (<= (`KismetMathLibrary.Vector_Distance` _returnvalue _returnvalue_2) (`self.AcceptanceRadius`))
      (bind _output_get (set `self.CurrentWaypointIndex` 1)))))

(fn `UserConstructionScript`)