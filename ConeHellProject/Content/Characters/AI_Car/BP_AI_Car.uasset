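; BP_AI_Car is an AI car actor that travels along a referenced spline and destroys itself after passing the end.
; Each Tick adds Speed times DeltaSeconds to a running distance, then moves the actor to that world-space point on SplineRef's spline.
; Movement sets location only, without sweep, so the car's rotation does not follow the spline.
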(event `self.ReceiveBeginPlay`)

(event `self.ReceiveTick`
  (params (DeltaSeconds :type "Float (single-precision)"))
  (bind _output_get (set `self.DistanceAlongSpline` (+ (* (`self.Speed`) DeltaSeconds) (`self.DistanceAlongSpline`))))
  (`self.K2_SetActorLocation` (+ (`SplineComponent.GetLocationAtDistanceAlongSpline` (`/Game/Characters/AI_Car/BP_Path.Spline` (`self.SplineRef`)) _output_get "World") (0.0 0.0 0.0)))
  (if (> (`self.DistanceAlongSpline`) (`SplineComponent.GetSplineLength` (`/Game/Characters/AI_Car/BP_Path.Spline` (`self.SplineRef`))))
    (`self.K2_DestroyActor`)))

(fn `UserConstructionScript`)